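; BP_AutoEODSkipper is a mod Blueprint that, by its name, is meant to auto-skip the end-of-day summary.
; While IsProcessingEOD is set, Tick casts the first top-level UserWidget to PlayHud and checks MHudState.EodPending.
; A pending state sets the same flag again; otherwise Tick calls ProcessEODSkip.
; ProcessEODSkip holds only an empty sequence, so no skip logic exists yet.
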(event `self.ReceiveBeginPlay`)

(event `self.ReceiveTick`
  (params (DeltaSeconds :type "Float (single-precision)"))
  (if (`self.IsProcessingEOD`)
    (bind _foundwidgets (`WidgetBlueprintLibrary.GetAllWidgetsOfClass` "/Script/UMG.UserWidget"))
    (bind _asplay_hud (cast `PlayHud` (`|GetArrayItem` _foundwidgets)))
    (bind _output_get (set `self.HudRef` _asplay_hud))
    (if (`.eodPending` (break `HudState` (`PlayHud.m_hudState` _output_get)))
      (set `self.IsProcessingEOD` true)
      (else
        (`self.ProcessEODSkip`)))))

(fn `ProcessEODSkip`
  (`|ExecutionSequence`))

(fn `UserConstructionScript`)